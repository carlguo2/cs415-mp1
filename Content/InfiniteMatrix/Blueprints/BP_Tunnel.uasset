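; BP_Tunnel is an endless-runner tunnel segment with a randomized, rotating holed wall that damages BP_Player on contact.
; Enemy count parity sets the spin direction.
; Entering TriggerZone makes TunnelSpawner spawn another segment, awards score unless the wall was hit, and destroys this one.
; Helper functions randomize the wall and chance-spawn health packs and enemies; end-overlap cleanup removes enemies only if a health pack is still valid.
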(event OnComponentBeginOverlap(TriggerZone)
  (params (OverlappedComponent :type Primitive%20Component%20Object%20Reference) (OtherActor :type Actor%20Object%20Reference) (OtherComp :type Primitive%20Component%20Object%20Reference) (OtherBodyIndex :type Integer) (bFromSweep :type Boolean) (SweepResult :type Hit%20Result%20Structure%20%28by%20ref%29))
  (bind _asbp_player (Utilities|Casting|CastToBP_Player OtherActor))
  (Default|SpawnTunnelatSpawnPoint (Variables|Default|GetTunnelSpawner))
  (if (Variables|/Game/InfiniteMatrix/Blueprints/BP_Player.BP_Player_C|GetIsWallCollided _asbp_player)
    (Variables|/Game/InfiniteMatrix/Blueprints/BP_Player.BP_Player_C|SetIsWallCollided _asbp_player false)
    (else
      (Default|AddScore _asbp_player)))
  (Actor|DestroyActor))

(event OnComponentBeginOverlap(WallMesh)
  (params (OverlappedComponent :type Primitive%20Component%20Object%20Reference) (OtherActor :type Actor%20Object%20Reference) (OtherComp :type Primitive%20Component%20Object%20Reference) (OtherBodyIndex :type Integer) (bFromSweep :type Boolean) (SweepResult :type Hit%20Result%20Structure%20%28by%20ref%29))
  (bind _asbp_player (Utilities|Casting|CastToBP_Player OtherActor))
  (Variables|/Game/InfiniteMatrix/Blueprints/BP_Player.BP_Player_C|SetIsWallCollided _asbp_player true)
  (Default|ReduceHealth _asbp_player 20))

(event OnComponentEndOverlap(TriggerZone)
  (params (OverlappedComponent :type Primitive%20Component%20Object%20Reference) (OtherActor :type Actor%20Object%20Reference) (OtherComp :type Primitive%20Component%20Object%20Reference) (OtherBodyIndex :type Integer))
  (bind _healthpack (Variables|Default|GetHealthPack))
  (Utilities|Casting|CastToBP_Player OtherActor)
  (if (Utilities|IsValid _healthpack)
    (Actor|DestroyActor _healthpack)
    (for _array_element (Variables|Default|GetEnemies)
      (if (Utilities|IsValid _array_element)
        (Actor|DestroyActor _array_element)))))

(event EventBeginPlay)

(event EventTick
  (params (DeltaSeconds :type Float%20%28single-precision%29))
  (bind _rotatespeed (Variables|Default|GetRotateSpeed))
  (bind _wallmesh (Variables|Default|GetWallMesh))
  (bind _returnvalue (* DeltaSeconds _rotatespeed))
  (if (== (Math|Integer|%(Integer) (Utilities|Array|Length (Variables|Default|GetEnemies)) 2) 0)
    (Transformation|AddLocalRotation _wallmesh (Math|Rotator|MakeRotator _returnvalue 0.0 0.0) false false)
    (else
      (bind _output_get (Variables|Default|SetBackwardRotateSpeed (* _returnvalue -1.0)))
      (Transformation|AddLocalRotation _wallmesh (Math|Rotator|MakeRotator _output_get 0.0 0.0) false false))))

(fn ConstructionScript)

(fn RandomizeWall
  (Components|StaticMesh|SetStaticMesh (Variables|Default|GetWallMesh) (Utilities|Select :Index (Math|Random|RandomIntegerinRange 0 3) :Option%200 "/Game/InfiniteMatrix/Meshes/SM_Hole_01.SM_Hole_01" :Option%201 "/Game/InfiniteMatrix/Meshes/SM_Hole_02.SM_Hole_02" :Option%202 "/Game/InfiniteMatrix/Meshes/SM_Hole_03.SM_Hole_03" :Option%203 "/Game/InfiniteMatrix/Meshes/SM_Hole_04.SM_Hole_04"))
  (Transformation|AddLocalRotation (Variables|Default|GetWallMesh) (Math|Rotator|MakeRotator (Math|Random|RandomFloatinRange 0.0 3.6e+02) 0.0 0.0) false false))

(fn SpawnHealthPack
  (params (TunnelSpawnVector :type Vector))
  (if (== (/ (Math|Random|RandomInteger 10) 3) 0)
    (bind _returnvalue (Game|SpawnActorfromClass "/Game/InfiniteMatrix/Blueprints/BP_HealthPack.BP_HealthPack_C" (Math|Transform|MakeTransform (Math|Vector|MakeVector (+ (.x TunnelSpawnVector) (Math|Random|RandomIntegerinRange 900 1300)) (+ (.y TunnelSpawnVector) (Math|Random|RandomIntegerinRange -250 250)) (+ (.z TunnelSpawnVector) (Math|Random|RandomIntegerinRange -250 250))) "0, 0, 0" "1.000000,1.000000,1.000000") "Undefined" "MultiplyWithRoot" 0 0))
    (Variables|Default|SetHealthPack _returnvalue)))

(fn SpawnEnemy
  (params (TunnelSpawnVector :type Vector))
  (if (< (Math|Random|RandomInteger 10) 3)
    (bind _returnvalue (Game|SpawnActorfromClass "/Game/InfiniteMatrix/Blueprints/BP_Enemy.BP_Enemy_C" (Math|Transform|MakeTransform (Math|Vector|MakeVector (+ (.x TunnelSpawnVector) (Math|Random|RandomIntegerinRange 900 1300)) (+ (.y TunnelSpawnVector) (Math|Random|RandomIntegerinRange -250 250)) (+ (.z TunnelSpawnVector) (Math|Random|RandomIntegerinRange -250 250))) "0, 0, 0" "1.000000,1.000000,1.000000") "Undefined" "MultiplyWithRoot" 0 0))
    (Utilities|Array|Add (Variables|Default|GetEnemies) _returnvalue)))